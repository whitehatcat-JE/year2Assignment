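; Enemy drone pawn that chases the player and explodes on contact.
; PawnSensing sightings trigger an AI move toward the player character, and overlapping it subtracts a fixed amount from its CurrentHealth.
; Incoming damage drains the drone's own EnemyHealth until it dies.
; Both contact and death by damage spawn an explosion, increment the player's EnemiesKilled and destroy the drone, so self-detonation also counts as a kill.
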(event OnSeePawn(PawnSensing)
  (params (Pawn :type Pawn%20Object%20Reference))
  ;[0 0 0] Scan for player
  (bind _asbp_third_person_character (Utilities|Casting|CastToBP_ThirdPersonCharacter (Game|GetPlayerCharacter 0)))
  (AI|AIMoveTo self "0, 0, 0" _asbp_third_person_character 1e+01 false))

(event Game|Damage|EventAnyDamage
  (params (Damage :type Float%20%28single-precision%29) (DamageType :type Damage%20Type%20Object%20Reference) (InstigatedBy :type Controller%20Object%20Reference) (DamageCauser :type Actor%20Object%20Reference))
  ;[0 0 0] Handles enemies taking damage
  (Variables|Default|SetEnemyHealth (- (Variables|Default|GetEnemyHealth) Damage))
  (if (<= (Variables|Default|GetEnemyHealth) 0.0)
    (bind _asbp_third_person_character (Utilities|Casting|CastToBP_ThirdPersonCharacter (Game|GetPlayerCharacter 0)))
    (Math|Integer|IncrementInt (Variables|/Game/ThirdPerson/Blueprints/BP_ThirdPersonCharacter.BP_ThirdPersonCharacter_C|GetEnemiesKilled _asbp_third_person_character)
      (:%20%20
        (Effects|SpawnEmitteratLocation "/Game/StarterContent/Particles/P_Explosion.P_Explosion" (Transformation|GetWorldLocation (Variables|Default|Getdrone)))
        (Actor|DestroyActor)))))

(event Collision|EventActorBeginOverlap
  (params (OtherActor :type Actor%20Object%20Reference))
  ;[0 0 0] Explodes on player collision
  (bind _asbp_third_person_character (Utilities|Casting|CastToBP_ThirdPersonCharacter OtherActor))
  (Variables|/Game/ThirdPerson/Blueprints/BP_ThirdPersonCharacter.BP_ThirdPersonCharacter_C|SetCurrent%20Health _asbp_third_person_character (- (Variables|/Game/ThirdPerson/Blueprints/BP_ThirdPersonCharacter.BP_ThirdPersonCharacter_C|GetCurrent%20Health _asbp_third_person_character) 75.0))
  (Effects|SpawnEmitteratLocation "/Game/StarterContent/Particles/P_Explosion.P_Explosion" (Transformation|GetWorldLocation (Variables|Default|Getdrone)))
  (bind _asbp_third_person_character_2 (Utilities|Casting|CastToBP_ThirdPersonCharacter (Game|GetPlayerCharacter 0)))
  (Math|Integer|IncrementInt (Variables|/Game/ThirdPerson/Blueprints/BP_ThirdPersonCharacter.BP_ThirdPersonCharacter_C|GetEnemiesKilled _asbp_third_person_character_2)
    (:%20%20
      (Actor|DestroyActor))))

(fn ConstructionScript)