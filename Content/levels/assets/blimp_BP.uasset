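; Blimp actor Blueprint that animates a spinning tail and propeller on the airship.
; BeginPlay picks a random speed multiplier so each instance spins at a slightly different rate.
; Tick sets both components' relative rotations from time since creation, wrapped to a full turn, with the propeller turning faster and opposite to the tail.
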(event EventBeginPlay
  (Variables|Default|SetrandomSpeedAdjustment (Math|Random|RandomFloatinRange 0.8 1.2)))

(event Collision|EventActorBeginOverlap
  (params (OtherActor :type Actor%20Object%20Reference)))

(event EventTick
  (params (DeltaSeconds :type Float%20%28single-precision%29))
  (bind _returnvalue (Actor|GetGameTimeSinceCreation))
  (bind _randomspeedadjustment (Variables|Default|GetrandomSpeedAdjustment))
  (Transformation|SetRelativeRotation (Variables|Default|GetblimpTail) (Math|Rotator|MakeRotator 9e+01 (Math|Float|%(Float) (* _returnvalue (* _randomspeedadjustment 5.0)) 3.6e+02) 0.0) false false)
  (Transformation|SetRelativeRotation (Variables|Default|GetblimpPropeller) (Math|Rotator|MakeRotator 9e+01 (- 3.6e+02 (Math|Float|%(Float) (* _returnvalue (* _randomspeedadjustment 5e+01)) 3.6e+02)) 0.0) false false))

(fn ConstructionScript)