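; Dome building Blueprint that animates six decorative gear components.
; Each Tick sets every gear's relative pitch directly from game time since creation, wrapped to 360 degrees, rather than accumulating rotation.
; Successive gears alternate direction and double in speed, mimicking a meshed gear train.
; The construction script is empty.
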(event EventTick
  (params (DeltaSeconds :type Float%20%28single-precision%29))
  (bind _returnvalue (Actor|GetGameTimeSinceCreation))
  ;[0 0 0] Rotate gears every frame
  (Transformation|SetRelativeRotation (Variables|Default|GetdomeGear1) (Math|Rotator|MakeRotator 0.0 (Math|Float|%(Float) (* _returnvalue 5.0) 3.6e+02) 0.0) false false)
  (Transformation|SetRelativeRotation (Variables|Default|GetdomeGear2) (Math|Rotator|MakeRotator 0.0 (- 3.6e+02 (Math|Float|%(Float) (* _returnvalue 1e+01) 3.6e+02)) 0.0) false false)
  (Transformation|SetRelativeRotation (Variables|Default|GetdomeGear3) (Math|Rotator|MakeRotator 0.0 (Math|Float|%(Float) (* _returnvalue 2e+01) 3.6e+02) 0.0) false false)
  (Transformation|SetRelativeRotation (Variables|Default|GetdomeGear4) (Math|Rotator|MakeRotator 0.0 (- 3.6e+02 (Math|Float|%(Float) (* _returnvalue 4e+01) 3.6e+02)) 0.0) false false)
  (Transformation|SetRelativeRotation (Variables|Default|GetdomeGear5) (Math|Rotator|MakeRotator 0.0 (Math|Float|%(Float) (* _returnvalue 8e+01) 3.6e+02) 0.0) false false)
  (Transformation|SetRelativeRotation (Variables|Default|GetdomeGear6) (Math|Rotator|MakeRotator 0.0 (- 3.6e+02 (Math|Float|%(Float) (* _returnvalue 1.6e+02) 3.6e+02)) 0.0) false false))

(fn ConstructionScript)