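; Exit tower double doors that stay shut until the player has killed a set total of enemies.
; Every Tick casts the player to BP_ThirdPersonCharacter, reads EnemiesKilled and shows the remaining count on EnemiesText.
; When kills exactly equal EnemiesTotal, it hides the text and calls OpenDoors on every such tick.
; OpenDoors plays a timeline that rotates both doors in opposite directions on pitch.
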(event Custom|openDoors
  ;[0 0 0] Open doors animation
  (bind _doorangle (Timeline|Timeline Play)
    (:Update
      (Transformation|SetRelativeRotation (Variables|Default|GetexitTowerDoorR) (Math|Rotator|MakeRotator 0.0 (* _doorangle -1.0) 0.0) false false)
      (Transformation|SetRelativeRotation (Variables|Default|GetexitTowerDoorL) (Math|Rotator|MakeRotator 0.0 _doorangle 0.0) false false))))

(event EventTick
  (params (DeltaSeconds :type Float%20%28single-precision%29))
  (bind _enemiestext (Variables|Default|GetenemiesText))
  (bind _enemiestotal (Variables|Default|GetEnemiesTotal))
  ;[0 0 0] Update displayed enemy counter and checks if open doors animation should play
  (bind _asbp_third_person_character (Utilities|Casting|CastToBP_ThirdPersonCharacter (Game|GetPlayerCharacter 0)))
  (bind _output_get (Variables|Default|SetEnemiesLeft (- _enemiestotal (Variables|/Game/ThirdPerson/Blueprints/BP_ThirdPersonCharacter.BP_ThirdPersonCharacter_C|GetEnemiesKilled _asbp_third_person_character))))
  (if (== (Variables|/Game/ThirdPerson/Blueprints/BP_ThirdPersonCharacter.BP_ThirdPersonCharacter_C|GetEnemiesKilled _asbp_third_person_character) _enemiestotal)
    (Rendering|SetVisibility _enemiestext false false)
    (CallFunction|OpenDoors)
    (else
      (Rendering|Components|TextRender|SetText _enemiestext (Utilities|Text|ToText(Integer) _output_get)))))

(fn ConstructionScript)