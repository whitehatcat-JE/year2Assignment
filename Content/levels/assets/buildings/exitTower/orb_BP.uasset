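; Exit tower orb Blueprint that continuously animates three decorative rings.
; Every Tick, it derives an angle from game time since creation, wrapped to a full turn, and sets each ring's relative rotation from it.
; The first and third rings spin on roll, while the second spins on yaw, all at the same constant speed.
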(event EventTick
  (params (DeltaSeconds :type Float%20%28single-precision%29))
  (bind _returnvalue (Actor|GetGameTimeSinceCreation))
  (bind _returnvalue_2 (* _returnvalue 1e+01))
  (bind _returnvalue_3 (Math|Float|%(Float) _returnvalue_2 3.6e+02))
  (Transformation|SetRelativeRotation (Variables|Default|GetexitTowerRing1) (Math|Rotator|MakeRotator _returnvalue_3 0.0 0.0) false false)
  (Transformation|SetRelativeRotation (Variables|Default|GetexitTowerRing2) (Math|Rotator|MakeRotator 0.0 0.0 _returnvalue_3) false false)
  (Transformation|SetRelativeRotation (Variables|Default|GetexitTowerRing3) (Math|Rotator|MakeRotator _returnvalue_3 0.0 0.0) false false))

(fn ConstructionScript)