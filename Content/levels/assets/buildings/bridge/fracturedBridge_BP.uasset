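; Fractured bridge building asset that animates three gear components as continuously spinning scenery.
; Every Tick sets each gear's relative pitch directly from game time since creation, wrapped to a full turn, so no rotation state is stored.
; Each gear turns twice as fast as the previous one, with the middle gear reversed to suggest meshed gearing.
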(event EventTick
  (params (DeltaSeconds :type Float%20%28single-precision%29))
  (bind _returnvalue (Actor|GetGameTimeSinceCreation))
  (Transformation|SetRelativeRotation (Variables|Default|GetfracteredBridgeGear1) (Math|Rotator|MakeRotator 0.0 (Math|Float|%(Float) (* _returnvalue 5.0) 3.6e+02) 0.0) false false)
  (Transformation|SetRelativeRotation (Variables|Default|GetfracteredBridgeGear2) (Math|Rotator|MakeRotator 0.0 (- 3.6e+02 (Math|Float|%(Float) (* _returnvalue 1e+01) 3.6e+02)) 0.0) false false)
  (Transformation|SetRelativeRotation (Variables|Default|GetfracteredBridgeGear3) (Math|Rotator|MakeRotator 0.0 (Math|Float|%(Float) (* _returnvalue 2e+01) 3.6e+02) 0.0) false false))

(fn ConstructionScript)